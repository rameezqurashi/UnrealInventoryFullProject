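; InventoryAsset_BP is a demo actor that exercises an Inventory system and prints the results on screen.
; The construction script sets stat and item name strings, which BeginPlay uses to register stats and item types with boost maps, consumable or equippable flags and placeholder textures.
; It then adds, consumes and equips sample items, and prints the equipped items and full inventory with flavor text and quantities.
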(event EventBeginPlay
  (bind _inventory (Variables|Default|GetInventory))
  ;[1 1 1] Add possible stats for inventory
  (Class|Inventory|AddPossibleStat (Variables|Default|GetInventory) (Variables|Default|GetAttackStatString))
  (Class|Inventory|AddPossibleStat (Variables|Default|GetInventory) (Variables|Default|GetDefenseStatString))
  (Class|Inventory|AddPossibleStat (Variables|Default|GetInventory) (Variables|Default|GetHPStatString))
  ;[1 1 1] Add possible inventory items
  (Class|Inventory|AddInventoryItemType _inventory (Variables|Default|GetSwordItemString) "A sword to attack your enemies!" "/Game/StarterContent/Textures/T_Brick_Clay_Beveled_D.T_Brick_Clay_Beveled_D" "/Game/StarterContent/Textures/T_Brick_Clay_Beveled_D.T_Brick_Clay_Beveled_D" (Utilities|Map|MakeMap (Variables|Default|GetAttackStatString) (Utilities|Struct|MakeBoostAndDuration 10)) 1 false true)
  (Class|Inventory|AddInventoryItemType _inventory (Variables|Default|GetSheildItemString) "A sheild to defend yourself!" "/Game/StarterContent/Textures/T_Burst_M.T_Burst_M" "/Game/StarterContent/Textures/T_Burst_M.T_Burst_M" (Utilities|Map|MakeMap (Variables|Default|GetDefenseStatString) (Utilities|Struct|MakeBoostAndDuration 10)) 1 false true)
  (Class|Inventory|AddInventoryItemType _inventory (Variables|Default|GetBreadItemString) "Bread to restore HP!" "/Game/StarterContent/Textures/T_Ceramic_Tile_M.T_Ceramic_Tile_M" "/Game/StarterContent/Textures/T_Ceramic_Tile_M.T_Ceramic_Tile_M" (Utilities|Map|MakeMap (Variables|Default|GetHPStatString) (Utilities|Struct|MakeBoostAndDuration 10)) 100 true false)
  (Class|Inventory|AddInventoryItemType _inventory (Variables|Default|GetSuperSheildItemString) "A better sheild to defend yourself!" "/Game/StarterContent/Textures/T_Fire_SubUV.T_Fire_SubUV" "/Game/StarterContent/Textures/T_Fire_SubUV.T_Fire_SubUV" (Utilities|Map|MakeMap (Variables|Default|GetHPStatString) (Utilities|Struct|MakeBoostAndDuration 15) (Variables|Default|GetDefenseStatString) (Utilities|Struct|MakeBoostAndDuration 15)) 1 false true)
  ;[1 1 1] Do some basic operations on the inventory
  (Class|Inventory|AddItem (Variables|Default|GetInventory) (Variables|Default|GetSwordItemString) 1)
  (Class|Inventory|AddItem (Variables|Default|GetInventory) (Variables|Default|GetBreadItemString) 5)
  (Class|Inventory|AddItem (Variables|Default|GetInventory) (Variables|Default|GetSheildItemString) 1)
  (Class|Inventory|ConsumeItem (Variables|Default|GetInventory) (Variables|Default|GetBreadItemString) 2)
  (Class|Inventory|EquipItem (Variables|Default|GetInventory) (Variables|Default|GetSwordItemString))
  ;[1 1 1] Print Equipped Items
  (Development|PrintString "Equipped Items Are:" true true "(R=0.000000,G=0.660000,B=1.000000,A=1.000000)" 1e+02)
  (bind _returnvalue (Class|Inventory|GetEquippedItems (Variables|Default|GetInventory)))
  (for _array_element _returnvalue
    (Development|PrintString (Utilities|String|Append (.Name (Utilities|Struct|BreakInventoryItem _array_element)) (.FlavorText (Utilities|Struct|BreakInventoryItem _array_element)) (Utilities|String|ToString(Integer) (.Quantity (Utilities|Struct|BreakInventoryItem _array_element)))) true true "(R=0.000000,G=0.660000,B=1.000000,A=1.000000)" 1e+02))
  ;[1 1 1] Print Whole Inventory
  (Development|PrintString "Complete Inventory Is:" true true "(R=0.000000,G=0.660000,B=1.000000,A=1.000000)" 1e+02)
  (bind _returnvalue_2 (Class|Inventory|GetInventory (Variables|Default|GetInventory)))
  (for _array_element_2 _returnvalue_2
    (Development|PrintString (Utilities|String|Append (.Name (Utilities|Struct|BreakInventoryItem _array_element_2)) (.FlavorText (Utilities|Struct|BreakInventoryItem _array_element_2)) (Utilities|String|ToString(Integer) (.Quantity (Utilities|Struct|BreakInventoryItem _array_element_2)))) true true "(R=0.000000,G=0.660000,B=1.000000,A=1.000000)" 1e+02)))

(fn ConstructionScript
  ;[1 1 1] Initialize Possible Stat Strings
  (Variables|Default|SetAttackStatString "Attack")
  (Variables|Default|SetDefenseStatString "Defense")
  (Variables|Default|SetHPStatString "HP")
  ;[1 1 1] Initialize Item Strings
  (Variables|Default|SetSwordItemString "Sword")
  (Variables|Default|SetSheildItemString "Sheild")
  (Variables|Default|SetBreadItemString "Bread")
  (Variables|Default|SetSuperSheildItemString "SuperSheild"))